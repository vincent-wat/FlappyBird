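; BP_Pipes is a pipe actor that scrolls along the world X axis while the player pawn, BP_Tony, is alive.
; Each Tick casts the player pawn to BP_Tony and checks its Dead flag, so movement halts once Tony dies.
; MovePipe applies a frame-rate independent, unswept offset from Speed, then KillPipe destroys the actor when its X drops below DespawnLocation.
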(event EventBeginPlay)

(event Collision|EventActorBeginOverlap
  (params (OtherActor :type Actor%20Object%20Reference)))

(event EventTick
  (params (DeltaSeconds :type Float%20%28single-precision%29))
  (bind _asbp_tony (Utilities|Casting|CastToBP_Tony (Game|Player|GetPlayerPawn 0)))
  (if (not (Variables|/Game/Blueprints/BP_Tony.BP_Tony_C|Getdead _asbp_tony))
    (CallFunction|MovePipe DeltaSeconds)
    (CallFunction|KillPipe)))

(fn ConstructionScript)

(fn MovePipe
  (params (DeltaSeconds :type Float%20%28double-precision%29))
  (Transformation|AddActorWorldOffset (Math|Vector|MakeVector (* DeltaSeconds (Variables|Default|GetSpeed)) 0.0 0.0)))

(fn KillPipe
  (if (< (.X (Math|Vector|BreakVector (Transformation|GetActorLocation))) (Variables|Default|GetDespawnLocation))
    (Actor|DestroyActor)))