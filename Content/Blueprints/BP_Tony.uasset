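; BP_Tony is the player-controlled bird in a Flappy Bird-style game, driven by physics on its Box component.
; While alive, a right mouse press zeroes the Box's velocity and applies an upward impulse.
; While it rises, Tick adds a small downward impulse and pitches the Box by its vertical velocity.
; Any hit sets Dead, blocking further flaps, and tells the BP_FlappyBird game mode to stop scoring.
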(event EventBeginPlay)

(event EventTick
  (params (DeltaSeconds :type Float%20%28single-precision%29))
  (bind _box (Variables|Default|GetBox))
  (bind _returnvalue (Physics|GetPhysicsLinearVelocity (Variables|Default|GetBox) "None"))
  (if (> (.z _returnvalue) 0.0)
    (Physics|AddImpulse _box "0.000000,0.000000,-15.000000" "None" false)
    (Transformation|SetRelativeRotation _box (Math|Rotator|MakeRotator 0.0 (/ (.z _returnvalue) 5e+01) 0.0) false false)))

(event Collision|EventHit
  (params (MyComp :type Primitive%20Component%20Object%20Reference) (Other :type Actor%20Object%20Reference) (OtherComp :type Primitive%20Component%20Object%20Reference) (bSelfMoved :type Boolean) (HitLocation :type Vector :default "0, 0, 0") (HitNormal :type Vector :default "0, 0, 0") (NormalImpulse :type Vector :default "0, 0, 0") (Hit :type Hit%20Result%20Structure%20%28by%20ref%29))
  (Variables|Default|Setdead true)
  (bind _asbp_flappy_bird (Utilities|Casting|CastToBP_FlappyBird (Game|GetGameMode)))
  (Default|StopScoring _asbp_flappy_bird))

(event Input|MouseEvents|RightMouseButton
  (params (Key :type Key%20Structure :default "None"))
  (bind _box (Variables|Default|GetBox))
  (:Pressed
    (if (not (Variables|Default|Getdead))
      (Physics|SetPhysicsLinearVelocity _box "0, 0, 0" false "None")
      (Physics|AddImpulse _box "0.000000,0.000000,550.000000" "None" false))))

(fn ConstructionScript)