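; BP_PipeSpawner is an actor that keeps spawning BP_Pipes obstacles during play, in what appears to be a Flappy Bird-style game.
; A looping timer started on BeginPlay calls SpawnPipe at a fixed interval.
; Each call spawns pipes at the spawner's X and Y with a random Z between MinHeight and MaxHeight, but only while the player pawn is a BP_Tony that is not dead.
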(event EventBeginPlay
  (Utilities|Time|SetTimerbyFunctionName 0 "SpawnPipe" 1.5 true))

(fn ConstructionScript)

(fn SpawnPipe
  (bind _returnvalue (Transformation|GetActorLocation))
  (bind (_x _y) (Math|Vector|BreakVector _returnvalue))
  (bind _asbp_tony (Utilities|Casting|CastToBP_Tony (Game|Player|GetPlayerPawn 0)))
  (if (not (Variables|/Game/Blueprints/BP_Tony.BP_Tony_C|Getdead _asbp_tony))
    (Game|SpawnActorfromClass "/Game/Blueprints/BP_Pipes.BP_Pipes_C" (Math|Conversions|ToTransform(Vector) (Math|Vector|MakeVector _x _y (Math|Random|RandomFloatinRange (Variables|Default|GetminHeight) (Variables|Default|GetmaxHeight)))) "Undefined" "MultiplyWithRoot" 0 0)))