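; Flappy Bird game mode that manages scoring, the score HUD and the saved high score.
; BeginPlay loads or creates the save game, sets game-only input, adds the HUD and starts a hardcoded delay before scoring begins.
; Score increments on a looping timer, so it tracks elapsed time rather than detecting obstacles passed.
; StopScoring clears that timer and saves the higher of the current score and stored high score.
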(event EventBeginPlay
  (bind _returnvalue (Game|GetPlayerController 0))
  (bind _returnvalue_2 (SaveGame|DoesSaveGameExist "1"))
  (if _returnvalue_2
    (bind _returnvalue_3 (SaveGame|LoadGamefromSlot "1"))
    (bind _asbp_save_game (Utilities|Casting|CastToBP_SaveGame _returnvalue_3))
    (Variables|Default|SetsaveGameRef _asbp_save_game)
    (else
      (bind _returnvalue_4 (SaveGame|CreateSaveGameObject "/Game/Blueprints/BP_SaveGame.BP_SaveGame_C"))
      (bind _output_get (Variables|Default|SetsaveGameRef _returnvalue_4))
      (SaveGame|SaveGametoSlot _output_get "1")))
  (Variables|/Script/Engine.PlayerController|SetbShowMouseCursor _returnvalue false)
  (Input|SetInputModeGameOnly _returnvalue false)
  (bind _returnvalue_5 (UserInterface|CreateWidget "/Game/Widgets/WBP_ScoreHud.WBP_ScoreHud_C")) ; Create a Widget Blueprint Object of our HUD to add it to the viewport. \nThis is a new BP for the Controller.
  (bind _output_get_2 (Variables|Default|SetscoreHUDRef _returnvalue_5))
  (UserInterface|Viewport|AddtoViewport _output_get_2 0)
  (Variables|Default|SetScore 0)
  (Utilities|Time|SetTimerbyFunctionName 0 "StartScoring" 2.6))

(event EventTick
  (params (DeltaSeconds :type Float%20%28single-precision%29)))

(fn ConstructionScript)

(fn StartScoring
  (bind _returnvalue (Utilities|Time|SetTimerbyFunctionName 0 "IncrementScore" 1.5 true))
  (Variables|Default|SetScoreTimerHandle _returnvalue))

(fn IncrementScore
  (Variables|Default|SetScore (+ 1 (Variables|Default|GetScore))))

(fn StopScoring
  (bind _savegameref (Variables|Default|GetsaveGameRef))
  (Utilities|Time|ClearandInvalidateTimerbyHandle (Variables|Default|GetScoreTimerHandle))
  (Variables|/Game/Blueprints/BP_SaveGame.BP_SaveGame_C|SethighScore _savegameref (Math|Integer|Max(Integer) (Variables|Default|GetScore) (Variables|/Game/Blueprints/BP_SaveGame.BP_SaveGame_C|GethighScore _savegameref)))
  (SaveGame|SaveGametoSlot _savegameref "1"))